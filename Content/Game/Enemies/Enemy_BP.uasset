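; Enemy Blueprint that handles the on-screen combat feedback: an overhead health bar and floating damage numbers.
; The health bar widget gets a reference to its enemy, starts hidden, toggles through parent show/hide events and rescales every Tick via HealthBarScaler.
; While not dying, hits spawn an animated number widget projected from world to screen, flagged for headshots, scaled likewise and registered through StoreHitNumber.
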(event EventBeginPlay
  ;[0 1 0.9208] BeginPlay and Initialize things
  (bind _asenemy_health_bar_bp (Utilities|Casting|CastToEnemyHealthBarBP (UserInterface|GetUserWidgetObject (Variables|Default|GetHealthBar))))
  (Variables|/Game/Game/HUD/EnemyHealthBarBP.EnemyHealthBarBP_C|SetEnemy_BP _asenemy_health_bar_bp self)
  (Widget|SetVisibility (UserInterface|GetUserWidgetObject (Variables|Default|GetHealthBar)) "Hidden"))

(event EventShowHealthBar
  ;[0.1472 0.2753 1] Show and Hide health bar
  (|CallParentFunction)
  (Widget|SetVisibility (UserInterface|GetUserWidgetObject (Variables|Default|GetHealthBar)) "Visible"))

(event EventHideHealthBar
  ;[0.1472 0.2753 1] Show and Hide health bar
  (|CallParentFunction)
  (Widget|SetVisibility (UserInterface|GetUserWidgetObject (Variables|Default|GetHealthBar)) "Hidden"))

(event EventTick
  (params (DeltaSeconds :type Float%20%28single-precision%29))
  (bind _returnvalue (Class|Enemy|HealthBarScaler))
  ;[1 0.1619 0] HealtBar Scaler and Event Tick
  (Widget|Transform|SetRenderScale (UserInterface|GetUserWidgetObject (Variables|Default|GetHealthBar)) (Math|Vector2D|MakeVector2D _returnvalue _returnvalue)))

(event EventShowHitNumber
  (params (Damage :type Integer) (HitLocation :type Vector :default "0, 0, 0") (bHeadShot :type Boolean))
  (bind _returnvalue (Class|Enemy|HealthBarScaler))
  (bind _returnvalue_2 (* _returnvalue 0.5))
  ;[0.9962 1 0] Damage Number Widget
  (if (not (Variables|Default|GetbDying))
    (Variables|Default|SetHit%20Location HitLocation)
    (Variables|Default|SetHead%20Shot bHeadShot)
    (bind _returnvalue_3 (UserInterface|CreateWidget "/Game/Game/HUD/HitNumber.HitNumber_C"))
    (bind _output_get (Variables|Default|SetWidgetRef _returnvalue_3))
    (Variables|/Game/Game/HUD/HitNumber.HitNumber_C|SetHitText _output_get (Utilities|Text|ToText(Integer) Damage))
    (UserInterface|Viewport|AddtoViewport (Variables|Default|GetWidgetRef) 0)
    (Class|UserWidget|SetPositioninViewport (Variables|Default|GetWidgetRef) (.ScreenPosition (Class|GameplayStatics|ProjectWorldtoScreen (Game|GetPlayerController 0) (Variables|Default|GetHit%20Location) false)) true)
    (Class|Enemy|StoreHitNumber (Variables|Default|GetWidgetRef) (Variables|Default|GetHit%20Location))
    (Variables|/Game/Game/HUD/HitNumber.HitNumber_C|SetHeadShot (Variables|Default|GetWidgetRef) (Variables|Default|GetHead%20Shot))
    (Widget|Transform|SetRenderScale (Variables|Default|GetWidgetRef) (Math|Vector2D|MakeVector2D _returnvalue_2 _returnvalue_2))
    (UserInterface|Animation|PlayAnimation (Variables|Default|GetWidgetRef) (Variables|/Game/Game/HUD/HitNumber.HitNumber_C|GetHitNumberAnimation (Variables|Default|GetWidgetRef)) 0.0 1 "Forward" 1.0 false)))

(fn ConstructionScript)