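; Belica's player character Blueprint, which detects when all enemies are defeated and shows a victory screen.
; BeginPlay gathers every Enemy_BP, then Tick polls their Dying flags into a parallel array, skipping invalid actors.
; Once no flag is false, a DoOnce creates the Yazi widget and plays its victory animation.
; Q runs a debug sphere trace from the follow camera, printing the hit actor's name, and Escape quits.
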(event EventBeginPlay
  ;[1 1 1] beginplay
  (bind _outactors (Actor|GetAllActorsOfClass "/Game/Game/Enemies/Enemy_BP.Enemy_BP_C"))
  (bind _output_get (Variables|Default|SetOut%20Actors _outactors))
  (for _array_element _output_get
    (Utilities|Array|Add (Variables|Default|GetIs%20Enemies%20Dying?) (Variables|/Script/Shooter.Enemy|GetbDying _array_element))))

(event EventTick
  (params (DeltaSeconds :type Float%20%28single-precision%29))
  (for (_array_element _array_index) (Variables|Default|GetOut%20Actors)
    (Utilities|IsValid _array_element
      (:Is%20Valid
        (Utilities|Array|SetArrayElem (Variables|Default|GetIs%20Enemies%20Dying?) _array_index (Variables|/Script/Shooter.Enemy|GetbDying _array_element)))))
  (if (not (Utilities|Array|ContainsItem (Variables|Default|GetIs%20Enemies%20Dying?) false))
    (Utilities|FlowControl|DoOnce false
      (:Completed
        (bind _returnvalue (UserInterface|CreateWidget "/Game/Game/HUD/Yazi.Yazi_C"))
        (UserInterface|Animation|PlayAnimation _returnvalue (Variables|/Game/Game/HUD/Yazi.Yazi_C|GetVictoryAnimation _returnvalue) 0.0 1 "Forward" 1.0 false)
        (UserInterface|Viewport|AddtoViewport _returnvalue 0)))))

(event Collision|EventActorBeginOverlap
  (params (OtherActor :type Actor%20Object%20Reference)))

(event Input|KeyboardEvents|Escape
  (params (Key :type Key%20Structure :default "None"))
  (:Pressed
    (Game|QuitGame 0 "Quit" false)))

(event Input|KeyboardEvents|Q
  (params (Key :type Key%20Structure :default "None"))
  (bind _followcamera (Variables|Default|GetFollowCamera))
  (bind _returnvalue (Transformation|GetWorldLocation _followcamera))
  (:Pressed
    (bind _outhits (Collision|MultiSphereTraceForObjects _returnvalue (+ _returnvalue (* (Math|Vector|GetForwardVector _followcamera) 5e+02)) 2e+01 (Utilities|Array|MakeArray "ObjectTypeQuery1") false (Utilities|Array|MakeArray self) "ForDuration"))
    (if (.bblockinghit (Utilities|Array|Get(acopy) _outhits))
      (Development|PrintString (Utilities|GetObjectName (.hitactor (Utilities|Array|Get(acopy) _outhits)))))))

(fn ConstructionScript)